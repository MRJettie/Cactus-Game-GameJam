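; BP_DamageNumber is a short-lived actor that shows a damage number in the world through a widget component.
; On BeginPlay it passes its DamageAmount to the WB_DamageText widget, then turns the component once to face the player camera using a look-at rotation flipped 180 degrees in yaw.
; It then sets a one-second lifespan to remove itself, which is skipped along with the rotation if the widget cast fails.
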(event EventBeginPlay
  (bind _widget (Variables|Default|GetWidget))
  (bind _aswb_damage_text (Utilities|Casting|CastToWB_DamageText (UserInterface|GetUserWidgetObject _widget)))
  (Default|SetDamageNumber _aswb_damage_text (Variables|Default|GetDamage%20Amount))
  (Transformation|SetWorldRotation _widget (Math|Rotator|CombineRotators (Math|Rotator|FindLookatRotation (Camera|GetCameraLocation (Game|GetPlayerCameraManager 0)) (Transformation|GetWorldLocation _widget)) "180.000000,0.000000,0.000000") false false)
  (Actor|SetLifeSpan 1.0))

(fn ConstructionScript)